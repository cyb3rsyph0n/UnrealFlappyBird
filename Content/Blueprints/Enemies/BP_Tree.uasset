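; BP_Tree is a scrolling tree obstacle with a bean sprite attached.
; On BeginPlay it randomizes its height if the game state is playing, otherwise it removes the bean.
; Tick moves it along negative X at a constant speed, regardless of play state.
; An overlapped bean destroys itself a tick later, and the whole actor is destroyed when Top1 overlaps an actor tagged "Boundry".
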(event OnComponentBeginOverlap(Sprite_Bean)
  (params (OverlappedComponent :type Primitive%20Component%20Object%20Reference) (OtherActor :type Actor%20Object%20Reference) (OtherComp :type Primitive%20Component%20Object%20Reference) (OtherBodyIndex :type Integer) (bFromSweep :type Boolean) (SweepResult :type Hit%20Result%20Structure%20%28by%20ref%29))
  (Utilities|IsValid OverlappedComponent
    (:Is%20Valid
      (Utilities|FlowControl|DelayUntilNextTick)
      (Components|DestroyComponent OverlappedComponent))))

(event OnComponentBeginOverlap(Top1)
  (params (OverlappedComponent :type Primitive%20Component%20Object%20Reference) (OtherActor :type Actor%20Object%20Reference) (OtherComp :type Primitive%20Component%20Object%20Reference) (OtherBodyIndex :type Integer) (bFromSweep :type Boolean) (SweepResult :type Hit%20Result%20Structure%20%28by%20ref%29))
  (if (Actor|ActorHasTag OtherActor "Boundry")
    (Actor|DestroyActor)))

(event EventTick
  (params (DeltaSeconds :type Float%20%28single-precision%29))
  (bind _returnvalue (Transformation|GetActorTransform))
  (Transformation|SetWorldLocation (Variables|Default|GetDefaultSceneRoot) (Math|Vector|MakeVector (+ (* DeltaSeconds -5e+02) (.x (.location _returnvalue))) (.y (.location _returnvalue)) (.z (.location _returnvalue))) false false))

(event EventBeginPlay
  (bind _returnvalue (Transformation|GetActorTransform))
  (bind _asbp_game_state (Utilities|Casting|CastToBP_GameState (Game|GetGameState)))
  (Variables|Default|SetCurrentState _asbp_game_state)
  (if (Variables|/Game/Blueprints/BP_GameState.BP_GameState_C|GetIsPlaying (Variables|Default|GetCurrentState))
    (Transformation|SetWorldLocation (Variables|Default|GetDefaultSceneRoot) (Math|Vector|MakeVector (.x (.location _returnvalue)) (.y (.location _returnvalue)) (Math|Random|RandomFloatinRange -8.3e+02 8.3e+02)) false false)
    (else
      (Components|DestroyComponent (Variables|Default|GetSprite_Bean)))))

(fn ConstructionScript)